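; Actor component that equips its owning Character with a weapon and handles firing, reloading, magazine checks and weapon cleanup.
; On BeginPlay it spawns the weapon class and snaps it to a mesh socket.
; Firing spends a round and aims at the target actor's location, but if that target's AI blackboard holds an owned cover, it randomly aims at either the head socket or below the actor's center.
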(event Custom|FireWeapon
  (params (TargetActor :type Actor%20Object%20Reference))
  (if (> (Variables|/Game/__BluePrints/BP_Rifle.BP_Rifle_C|GetCurMegazine (Variables|Default|GetWeaponRef)) 0)
    (bind _result (Math|Integer|DecrementInt (Variables|/Game/__BluePrints/BP_Rifle.BP_Rifle_C|GetCurMegazine (Variables|Default|GetWeaponRef)))
      (:%20%20
        (Variables|Default|SetAttackTargetCache TargetActor)
        (if (Utilities|IsValid (AI|Components|Blackboard|GetValueasObject (AI|GetBlackboard (AI|GetAIController (Variables|Default|GetAttackTargetCache))) (Variables|Default|GetOwnedCoverKeyName)))
          (if (> (Math|Random|RandomIntegerinRange 0 100) 50)
            (bind _ascharacter (Utilities|Casting|CastToCharacter (Variables|Default|GetAttackTargetCache)))
            (Default|Fire (Variables|Default|GetWeaponRef) (Transformation|GetSocketLocation (Variables|/Script/Engine.Character|GetMesh _ascharacter) (Variables|Default|GetTargetHeadSocketName)))
            (else
              (Default|Fire (Variables|Default|GetWeaponRef) (- (Transformation|GetActorLocation (Variables|Default|GetAttackTargetCache)) "0.000000,0.000000,50.000000"))))
          (else
            (Default|Fire (Variables|Default|GetWeaponRef) (Transformation|GetActorLocation (Variables|Default|GetAttackTargetCache)))))))))

(event Custom|OnDestroy
  (Actor|DestroyActor (Variables|Default|GetWeaponRef)))

(event Custom|Reload
  (bind _weaponref (Variables|Default|GetWeaponRef))
  (Variables|/Game/__BluePrints/BP_Rifle.BP_Rifle_C|SetCurMegazine _weaponref (Variables|/Game/__BluePrints/BP_Rifle.BP_Rifle_C|GetMaxMegazine _weaponref)))

(event EventBeginPlay
  (bind _ascharacter (Utilities|Casting|CastToCharacter (Components|GetOwner)))
  (Variables|Default|SetCharacterRef _ascharacter)
  (CallFunction|EquipWeapon))

(fn EquipWeapon
  (bind _returnvalue (Game|SpawnActorfromClass (Variables|Default|GetWeaponClass) (Math|Transform|MakeTransform "0, 0, 0" "0, 0, 0" "1.000000,1.000000,1.000000") "Undefined" "MultiplyWithRoot" 0 0))
  (bind _output_get (Variables|Default|SetWeaponRef _returnvalue))
  (Transformation|AttachComponentToComponent _output_get (Variables|/Script/Engine.Character|GetMesh (Variables|Default|GetCharacterRef)) (Variables|Default|GetWeaponSocketName) "SnapToTarget" "SnapToTarget" "SnapToTarget" true))

(fn IsMegazineEmpty
  (return (<= (Variables|/Game/__BluePrints/BP_Rifle.BP_Rifle_C|GetCurMegazine (Variables|Default|GetWeaponRef)) 0)))