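; BP_Enemy is an AI enemy character Blueprint with weapon and stat components.
; BeginPlay, damage, fire and reload events only forward to the parent class, which holds the actual behavior.
; The CharacterStat Die event just casts the controller to AIC_Enemy.
; Weapon cleanup, controller death notification, game mode deregistration and actor destruction are present but disconnected, so they never run here.
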(event Die(CharacterStat)
  (bind _asaic_enemy (Utilities|Casting|CastToAIC_Enemy (Pawn|GetController))))

(event EventFire
  (params (TargetActor :type Actor%20Object%20Reference))
  (|CallParentFunction TargetActor))

(event EventReload
  (|CallParentFunction))

(event EventBeginPlay
  (|CallParentFunction))

(event EventGetDamage
  (params (DamageAmount :type Integer))
  (|CallParentFunction DamageAmount))

(fn ConstructionScript)