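; Actor component that manages activation and cooldown of a passive skill for its owner.
; ActivatePassive spawns an actor of PassiveClass, sets the owner as its caster and caches that actor's duration and cool time.
; Tick counts down the duration first and only then the cooldown, clearing the activated flag when both expire.
; IsSkillAvailable reports whether the cooldown has run out.
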(event Custom|ActivatePassive
  (bind _returnvalue (Game|SpawnActorfromClass (Variables|Default|GetPassiveClass) (Math|Transform|MakeTransform "0, 0, 0" "0, 0, 0" "1.000000,1.000000,1.000000") "Undefined" "MultiplyWithRoot" 0 0))
  (Variables|/Game/__BluePrints/BP_PassiveSkill.BP_PassiveSkill_C|SetCasterRef _returnvalue (Components|GetOwner))
  (Variables|Default|SetIsActivated true)
  (Variables|Default|SetCoolDown (Variables|/Game/__BluePrints/BP_PassiveSkill.BP_PassiveSkill_C|GetCoolTime _returnvalue))
  (Variables|Default|SetDurationCache (Variables|/Game/__BluePrints/BP_PassiveSkill.BP_PassiveSkill_C|GetDuration _returnvalue)))

(event EventTick
  (params (DeltaSeconds :type Float%20%28single-precision%29))
  (if (Variables|Default|GetIsActivated)
    (bind _output_get (Variables|Default|SetDurationCache (- (Variables|Default|GetDurationCache) DeltaSeconds)))
    (if (<= _output_get 0.0)
      (bind _output_get_2 (Variables|Default|SetCoolDown (- (Variables|Default|GetCoolDown) DeltaSeconds)))
      (if (<= _output_get_2 0.0)
        (Variables|Default|SetIsActivated false)))))

(fn IsSkillAvailable
  (return (<= (Variables|Default|GetCoolDown) 0.0)))