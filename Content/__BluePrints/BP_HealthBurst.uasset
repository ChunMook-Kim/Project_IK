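; Health burst skill actor that heals its caster, which must be a BP_PassiveSkillGunner, over a set duration.
; After calling parent BeginPlay, it casts the caster reference, sets the heal timeline's length to Duration and plays it.
; Each timeline update adds the curve's heal amount to the caster's hit points and truncates the total, so healing depends on update frequency.
; The actor destroys itself when the timeline finishes.
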(event EventTick
  (params (DeltaSeconds :type Float%20%28single-precision%29))
  (|CallParentFunction)
  (bind _asbp_passive_skill_gunner (Utilities|Casting|CastToBP_PassiveSkillGunner (Variables|Default|GetCasterRef)))
  (Variables|Default|SetPassiveSkillGunnerRef _asbp_passive_skill_gunner)
  (Components|Timeline|SetTimelineLength (Variables|Default|GetHealTimeline) (Variables|Default|GetDuration))
  (bind _healamount (Timeline|HealTimeline Play)
    (:Update
      (Class|CharacterStatComponent|SetHitPoint (Variables|/Game/__BluePrints/BP_Gunner.BP_Gunner_C|GetCharacterStat (Variables|Default|GetPassiveSkillGunnerRef)) (Math|Conversions|ToFloat(Integer) (Math|Float|Truncate (+ _healamount (Class|CharacterStatComponent|GetHitPoint (Variables|/Game/__BluePrints/BP_Gunner.BP_Gunner_C|GetCharacterStat (Variables|Default|GetPassiveSkillGunnerRef))))))))
    (:Finished
      (Actor|DestroyActor))))

(fn ConstructionScript
  (|CallParentFunction))