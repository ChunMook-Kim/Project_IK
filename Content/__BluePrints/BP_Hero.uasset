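; Hero Blueprint that fires bullets and visualises its detection and firing ranges.
; Each tick, DebugDraw draws circles at the actor's location for SightRange, colored red or green by IsNoticeEnemy, and for FireRange.
; The Fire event spawns BP_Bullet using MuzzleTransform, which is meant to offset the spawn point along the forward vector.
; Enemy detection and the trigger for Fire are not implemented in these graphs.
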(event Custom|Fire
  (Game|SpawnActorfromClass "/Game/__BluePrints/BP_Bullet.BP_Bullet_C" (Utilities|MuzzleTransform) "Undefined" "MultiplyWithRoot" 0 0))

(event EventTick
  (params (DeltaSeconds :type Float%20%28single-precision%29))
  (Utilities|DebugDraw))

(fn ConstructionScript)